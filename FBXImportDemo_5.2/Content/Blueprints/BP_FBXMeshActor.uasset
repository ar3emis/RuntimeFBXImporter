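; Selectable FBX mesh actor that shows UI for browsing its node hierarchy and editing the materials of its mesh sections.
; Actor selection opens a tree view of the root nodes, kept in sync both ways with component selection; selection reset removes both widgets.
; Received section data fills a lazily created section menu, whose events apply material, diffuse texture and diffuse color changes to the current component.
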(event Custom|OnMaterialSelected_Event
  (params (SectionID :type Integer) (Material :type Material%20Interface%20Object%20Reference))
  ;[1 1 1] Update Material Parameters
  (Class|FBXMeshActor|UpdateSectionMaterial SectionID Material (Variables|Default|GetCurrentComponent)))

(event Custom|OnTextureSelected_Event
  (params (SectionID :type Integer) (Texture :type Texture%202D%20Object%20Reference))
  ;[1 1 1] Update Material Parameters
  (Class|FBXMeshActor|UpdateTextureParameter SectionID "DIffuseTexture" Texture (Variables|Default|GetCurrentComponent)))

(event Custom|OnSectionColorChanged_Event
  (params (SectionID :type Integer) (NewColor :type Linear%20Color%20Structure))
  ;[1 1 1] Update Material Parameters
  (Class|FBXMeshActor|UpdateVectorParameter SectionID "DiffuseColor" NewColor (Variables|Default|GetCurrentComponent)))

(event Custom|OnRowSelected_Event
  (params (SelectedNode :type Mesh%20Node%20Object%20Reference))
  (Class|FBXMeshActor|SelectComponentfromMeshNode SelectedNode))

(event EventOnActorSelectionReset
  (bind _treeviewwidget (Variables|Default|GetTreeViewWidget))
  (bind _sectionmenu (Variables|Default|GetSectionMenu))
  ;[1 0.2774 0] On Actor Selection Reset
  (Utilities|FlowControl|Sequence
    (:then_0
      (Utilities|IsValid _treeviewwidget
        (:Is%20Valid
          (Widget|RemovefromParent _treeviewwidget))))
    (:then_1
      (Utilities|IsValid _sectionmenu
        (:Is%20Valid
          (Widget|RemovefromParent _sectionmenu))))))

(event EventOnActorSelected
  ;[0 1 0.4593] On Actor Selected
  (Utilities|IsValid (Variables|Default|GetTreeViewWidget)
    (:Is%20Valid
      (if (not (UserInterface|Viewport|IsinViewport (Variables|Default|GetTreeViewWidget)))
        (UserInterface|Viewport|AddtoViewport (Variables|Default|GetTreeViewWidget) 0 :!label _label)
        (EventDispatchers|AssignOnRowSelected (Variables|Default|GetTreeViewWidget) (delegate Custom|OnRowSelected_Event))))
    (:Is%20Not%20Valid
      (bind _returnvalue (UserInterface|CreateWidget "/Game/Widgets/TreeView/UMG_TreeView.UMG_TreeView_C" 0 (Class|FBXMeshActor|GetRootNodes)))
      (Variables|Default|SetTreeViewWidget _returnvalue)
      (goto _label))))

(event EventOnComponentHovered
  (params (MeshComponent :type Procedural%20Mesh%20Component%20Object%20Reference)))

(event EventOnComponentSelected
  (params (MeshComponent :type Procedural%20Mesh%20Component%20Object%20Reference))
  (bind _treeviewwidget (Variables|Default|GetTreeViewWidget))
  (Variables|Default|SetCurrentComponent MeshComponent)
  (Utilities|IsValid _treeviewwidget
    (:Is%20Valid
      (Default|HighlightandExpandNode _treeviewwidget (Class|FBXMeshActor|GetMeshNodefromComponent MeshComponent)))))

(event EventOnSectionReceived
  (params (SectionData :type Array%20of%20Procedural%20Mesh%20Data%20Structures) (MaterialInfo :type Array%20of%20Material%20Info%20Structures) (TextureInfo :type Array%20of%20Texture%20Info%20Structures))
  ;[0.5513 0.149 1] On Section Received
  (Utilities|FlowControl|Sequence
    (:then_0
      (Utilities|IsValid (Variables|Default|GetSectionMenu)
        (:Is%20Not%20Valid
          (bind _returnvalue (UserInterface|CreateWidget "/Game/Widgets/MenWidgets/UMG_SectionMenu.UMG_SectionMenu_C" 0 MaterialInfo TextureInfo))
          (bind _output_get (Variables|Default|SetSectionMenu _returnvalue))
          ;[1 1 1] Update Material Parameters
          (EventDispatchers|AssignOnMaterialSelected _output_get (delegate Custom|OnMaterialSelected_Event))
          (EventDispatchers|AssignOnTextureSelected (Variables|Default|GetSectionMenu) (delegate Custom|OnTextureSelected_Event))
          (EventDispatchers|AssignOnSectionColorChanged (Variables|Default|GetSectionMenu) (delegate Custom|OnSectionColorChanged_Event)))))
    (:then_1
      (if (UserInterface|Viewport|IsinViewport (Variables|Default|GetSectionMenu))
        _
        (else
          (UserInterface|Viewport|AddtoViewport (Variables|Default|GetSectionMenu) 0)))
      (Default|UpdateSectionData (Variables|Default|GetSectionMenu) SectionData))))

(fn ConstructionScript)